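; BP_GS_Timer, likely a Game State, keeps a count of elapsed seconds for the timer game mode.
; On BeginPlay it takes the player controller from BP_GM_Timer, resets the count and starts a looping one-second timer.
; Each tick increments the count and sends it to the controller's update call.
; It binds to the game mode's stop-timer dispatcher, evidently so StopTimer can clear the timer handle.
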(event Custom|TimerIncrement
  (bind _output_get (Variables|Default|SetTimer (+ (Variables|Default|GetTimer) 1)))
  (Default|CallUpdateTimer (Variables|Default|GetPlayer%20Controller) _output_get))

(event Custom|StopTimer
  (Utilities|Time|ClearandInvalidateTimerbyHandle (Variables|Default|GetTimerHandleRef)))

(event EventBeginPlay
  (bind _asbp_gm_timer (Utilities|Casting|CastToBP_GM_Timer (Game|GetGameMode)))
  (bind _output_get (Variables|Default|SetAs%20BP%20GM%20Timer _asbp_gm_timer))
  (Variables|Default|SetPlayer%20Controller (Variables|/Game/Blueprints/_Game/BP_GM_Timer.BP_GM_Timer_C|GetPlayerController _output_get))
  (Variables|Default|SetTimer 0)
  (bind _returnvalue (Utilities|Time|SetTimerbyEvent (EventDispatchers|CreateEvent :!event Custom|TimerIncrement) 1.0 true))
  (Variables|Default|SetTimerHandleRef _returnvalue)
  (EventDispatchers|BindEventtoHandleStopTimer (Variables|Default|GetAs%20BP%20GM%20Timer) (EventDispatchers|CreateEvent :!event Custom|StopTimer)))

(fn ConstructionScript)