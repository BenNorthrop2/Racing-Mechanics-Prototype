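; Game mode for a timed trolley-collection level, counting elapsed seconds and trolleys and opening a level once the count reaches the maximum.
; On BeginPlay it starts a looping timer, binds trolley increment and bay registration events, then after a short delay tells each registered bay to spawn a random trolley share.
; Timer and counter changes are pushed to the player controller.
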(event Custom|TimerIncrement
  (bind _output_get (Variables|Default|SetTimer (+ (Variables|Default|GetTimer) 1)))
  (Default|CallUpdateTimer (Variables|Default|GetPlayerController) _output_get))

(event Custom|AddTrolley
  (bind _output_get (Variables|Default|SetCurrentTrolleys (+ (Variables|Default|GetCurrentTrolleys) 1)))
  (Default|CallUpdateTrolleyCounter (Variables|Default|GetPlayerController) (Variables|Default|GetCurrentTrolleys) (Variables|Default|GetMaxTrolleys))
  (if (== _output_get (Variables|Default|GetMaxTrolleys))
    (Game|OpenLevel(byObjectReference) "/Game/Levels/LevelSelect.LevelSelect")))

(event Custom|AddTrolleyBay
  (params (TrolleyBay :type Actor%20Object%20Reference))
  (Utilities|Array|AddUnique (Variables|Default|GetTrolleyBays) TrolleyBay))

(event EventBeginPlay
  (bind _trolleybays (Variables|Default|GetTrolleyBays))
  (bind _maxtrolleys (Variables|Default|GetMaxTrolleys))
  (bind _returnvalue (Utilities|Array|Length _trolleybays))
  (bind _returnvalue_2 (/ _maxtrolleys _returnvalue))
  (bind _returnvalue_3 (Math|Random|RandomIntegerinRange 0 _returnvalue_2))
  (bind _asbp_pc_player (Utilities|Casting|CastToBP_PC_Player (Game|GetPlayerController 0)))
  (Variables|Default|SetPlayerController _asbp_pc_player)
  (Variables|Default|SetTimer 0)
  (Utilities|Time|SetTimerbyEvent (EventDispatchers|CreateEvent :!event Custom|TimerIncrement) 1.0 true)
  (EventDispatchers|BindEventtoHandleIncrementTrolley (EventDispatchers|CreateEvent :!event Custom|AddTrolley))
  (Utilities|FlowControl|DelayUntilNextTick)
  (EventDispatchers|BindEventtoHandleGetTrolleyBays (delegate Custom|AddTrolleyBay))
  (Utilities|FlowControl|Delay 1.0)
  (Variables|Default|SetTrolleysToSpawn (Variables|Default|GetMaxTrolleys))
  (for _array_element _trolleybays
    (Variables|Default|SetTrolleysToSpawn (- (Variables|Default|GetTrolleysToSpawn) _returnvalue_3))
    (Class|BPITrolleyBay|SpawnTrolley(Message) _array_element _returnvalue_3))
  (Development|PrintString (Utilities|String|ToString(Integer) 0))
  (Default|CallUpdateTrolleyCounter (Variables|Default|GetPlayerController) (Variables|Default|GetCurrentTrolleys) (Variables|Default|GetMaxTrolleys)))

(fn ConstructionScript)

(fn SpawnTrolleys
  (params (Trolley%20Actor :type Actor%20Class%20Reference) (Spawn%20Transform :type Transform))
  (Game|SpawnActorfromClass Trolley%20Actor Spawn%20Transform "Undefined" "MultiplyWithRoot" 0 0)
  (Math|Integer|IncrementInt (Variables|Default|GetCurrentTrolleys)))

(fn GetGameModeRef
  (return self))