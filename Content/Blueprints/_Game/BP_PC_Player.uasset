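; Player controller that sets up the player's input and owns the gameplay HUD and end screen widgets.
; On BeginPlay it adds the Enhanced Input player mapping context, switches to game-only input, and creates both widgets, keeping the end screen collapsed.
; Events hide the game UI or reveal the end screen, the latter switching to UI-only input with the mouse cursor shown.
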(event Custom|HideGameUI
  (Widget|SetVisibility (Variables|Default|GetGameplayWidget) "Collapsed"))

(event Custom|ShowEndScreenUI
  (bind _endscreenwidget (Variables|Default|GetEndScreenWidget))
  (Widget|SetVisibility _endscreenwidget "Visible")
  (Input|SetInputModeUIOnly self _endscreenwidget "DoNotLock" false)
  (Variables|Default|SetbShowMouseCursor true))

(event EventBeginPlay
  (bind _self self)
  (bind _returnvalue (PlayerController|LocalPlayerSubsystems|GetEnhancedInputLocalPlayerSubsystem _self))
  (Utilities|IsValid _returnvalue
    (:Is%20Valid
      (Input|AddMappingContext _returnvalue "/Game/Blueprints/_Game/Input/IMC_Player.IMC_Player" 0 "(bIgnoreAllPressedKeysUntilRelease=True,bForceImmediately=False,bNotifyUserSettings=False)")
      (Input|SetInputModeGameOnly self false)
      ;[0.15 0.15 0.15 0.5] UI
      (bind _returnvalue_2 (UserInterface|CreateWidget "/Game/Blueprints/_Game/UI/WBP_GameUI.WBP_GameUI_C" self))
      (bind _output_get (Variables|Default|SetGameplayWidget _returnvalue_2))
      (Variables|/Game/Blueprints/_Game/UI/WBP_GameUI.WBP_GameUI_C|SetPlayerController _output_get self)
      (bind _returnvalue_3 (UserInterface|CreateWidget "/Game/Blueprints/_Game/UI/WBP_EndScreen.WBP_EndScreen_C" self))
      (bind _output_get_2 (Variables|Default|SetEndScreenWidget _returnvalue_3))
      (Widget|SetVisibility _output_get_2 "Collapsed")
      (UserInterface|Viewport|AddtoViewport (Variables|Default|GetGameplayWidget) 0))))

(fn ConstructionScript)