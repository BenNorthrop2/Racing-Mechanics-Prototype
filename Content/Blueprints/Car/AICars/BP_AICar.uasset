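; AI car Blueprint that drives along a spline, with a random mesh and chassis colour picked at construction.
; A looping timer updates movement, steering by yaw to the target spline point and scaling throttle by that point's distance along the spline.
; The target index advances when the car gets close, reversing direction at either end of the spline to ping-pong along it.
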(event Custom|UpdateMovement
  (bind _followspline (Variables|Default|GetFollowSpline))
  (Utilities|IsValid _followspline
    (:Is%20Valid
      (bind _steering (CallFunction|GetSteeringAlongSpline _followspline))
      (Class|ChaosVehicleMovementComponent|SetSteeringInput (Variables|Default|GetVehicleMovementComponent) _steering)
      (Class|ChaosVehicleMovementComponent|SetThrottleInput (Variables|Default|GetVehicleMovementComponent) (Math|Float|MapRangeClamped (Spline|GetDistanceAlongSplineatSplinePoint (Variables|Default|GetFollowSpline) (Variables|Default|GetPointIndex)) 1.5e+03 2e+02 1.0 0.2))
      (if (< (Math|Vector|Distance(Vector) (Spline|GetLocationatSplinePoint (Variables|Default|GetFollowSpline) (Variables|Default|GetPointIndex) "World") (Transformation|GetActorLocation)) 8e+02)
        (CallFunction|IncrementPoint)))))

(event EventBeginPlay
  (Utilities|FlowControl|DelayUntilNextTick)
  (Utilities|Time|SetTimerbyEvent (EventDispatchers|CreateEvent :!event Custom|UpdateMovement) 0.1 true))

(fn ConstructionScript
  (bind _mesh (Variables|Character|GetMesh))
  (Components|SkeletalMesh|SetSkeletalMeshAsset _mesh (.OutItem (Utilities|Array|Random (Variables|Default|GetCarMeshes))))
  (bind _returnvalue (Rendering|Material|CreateDynamicMaterialInstance _mesh 1 "/Game/Assets/Cars/Materials/MI_ChasisColour.MI_ChasisColour" "None" :!class /Script/Engine.PrimitiveComponent))
  (bind _output_get (Variables|Default|SetMaterial _returnvalue))
  (Rendering|Material|SetVectorParameterValue _output_get "Chasis_Colour" (.OutItem (Utilities|Array|Random (Variables|Default|GetCarColours))) :!class /Script/Engine.MaterialInstanceDynamic))

(fn GetSteeringAlongSpline
  (params (Spline :type Spline%20Component%20Object%20Reference))
  (return (Math|Float|MapRangeClamped (.yaw (Math|Rotator|Delta(Rotator) (Math|Rotator|FindLookatRotation (Transformation|GetActorLocation) (Spline|GetLocationatSplinePoint Spline (Variables|Default|GetPointIndex) "World")) (Transformation|GetActorRotation))) -2e+01 2e+01 -1.0 1.0)))

(fn IncrementPoint
  (bind _output_get (Variables|Default|SetPointIndex (+ (Variables|Default|GetPointIndex) (Variables|Default|GetDirection))))
  (if (== _output_get (- (Spline|GetNumberOfSplinePoints (Variables|Default|GetFollowSpline)) 1))
    (Variables|Default|SetDirection -1)
    (elif (== (Variables|Default|GetPointIndex) 0)
      (Variables|Default|SetDirection 1))))