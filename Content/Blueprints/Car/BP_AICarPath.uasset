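; BP_AICarPath is a spline path actor that populates itself with AI cars.
; On BeginPlay it spawns a BP_AICar at the spline's start, handing it the spline and Loop flag.
; SpawnCars re-calls itself after a short random delay to stagger cars until MaxCars is reached, stopping early if a spawn fails.
; GetSpline exposes the spline to other Blueprints.
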(event Custom|SpawnCars
  (if (not (== (Variables|Default|GetCarsSpawned) (Variables|Default|GetMaxCars)))
    (bind _returnvalue (Game|SpawnActorfromClass "/Game/Blueprints/Car/AICars/BP_AICar.BP_AICar_C" (Math|Transform|MakeTransform (Spline|GetLocationatDistanceAlongSpline (Variables|Default|GetSpline) 0.0 "World") (Spline|GetRotationatDistanceAlongSpline (Variables|Default|GetSpline) 0.0 "World") "1.000000,1.000000,1.000000") "AdjustIfPossibleButAlwaysSpawn" "MultiplyWithRoot" 0 (Variables|Default|GetSpline) (Variables|Default|GetLoop?) 0))
    (Utilities|IsValid _returnvalue
      (:Is%20Valid
        (Math|Integer|IncrementInt (Variables|Default|GetCarsSpawned)
          (:%20%20
            (Utilities|FlowControl|Delay (Math|Random|RandomFloatinRange 2.0 3.0))
            (CallFunction|SpawnCars)))))))

(event EventBeginPlay
  (CallFunction|SpawnCars))

(fn ConstructionScript)

(fn GetSpline
  (return (Variables|Default|GetSpline)))