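; Player character with look, camera-relative movement and sprint that can take control of trolleys and return on foot.
; Interact runs a sphere trace around the player and, through BPI_TrolleyInterface, asks an unconnected trolley to be possessed, then hides the mesh and disables collision.
; ReturntoPlayer stores the trolley and repossesses the player, whose Possessed event teleports it to the trolley's handlebar and restores visibility and query-and-probe collision.
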(event Input|EnhancedActionEvents|EnhancedInputActionIA_Look
  (params (ActionValue :type Vector%202D%20Structure) (ElapsedSeconds :type Float%20%28double-precision%29) (TriggeredSeconds :type Float%20%28double-precision%29) (InputAction :type Input%20Action%20Object%20Reference :default "/Game/Blueprints/_Game/Input/Inputs/Movement/IA_Look.IA_Look"))
  (Pawn|Input|AddControllerYawInput (.x ActionValue))
  (Pawn|Input|AddControllerPitchInput (.y ActionValue)))

(event Input|EnhancedActionEvents|EnhancedInputActionIA_Move
  (params (ActionValue :type Vector%202D%20Structure) (ElapsedSeconds :type Float%20%28double-precision%29) (TriggeredSeconds :type Float%20%28double-precision%29) (InputAction :type Input%20Action%20Object%20Reference :default "/Game/Blueprints/_Game/Input/Inputs/Movement/IA_Move.IA_Move"))
  (Pawn|Input|AddMovementInput (Math|Vector|GetRightVector (Math|Rotator|MakeRotator 0.0 0.0 (.yaw (Pawn|GetControlRotation :!class /Script/Engine.Pawn)))) (.x ActionValue) false)
  (Pawn|Input|AddMovementInput (Math|Vector|GetForwardVector (Math|Rotator|MakeRotator 0.0 0.0 (.yaw (Pawn|GetControlRotation :!class /Script/Engine.Pawn)))) (.y ActionValue) false))

(event Input|EnhancedActionEvents|EnhancedInputActionIA_Interact
  (params (ActionValue :type Boolean) (ElapsedSeconds :type Float%20%28double-precision%29) (TriggeredSeconds :type Float%20%28double-precision%29) (InputAction :type Input%20Action%20Object%20Reference :default "/Game/Blueprints/_Game/Input/Inputs/Abilities/IA_Interact.IA_Interact"))
  (bind _returnvalue (Transformation|GetActorLocation))
  (bind _outhit (Collision|SphereTraceByChannel _returnvalue _returnvalue 2e+02 "TraceTypeQuery1" false 0 "ForDuration"))
  (if (Utilities|DoesObjectImplementInterface (.HitActor (Collision|BreakHitResult _outhit)) "/Game/Blueprints/Interfaces/BPI_TrolleyInterface.BPI_TrolleyInterface_C")
    (bind _success (Class|BPITrolleyInterface|CheckConnection(Message) (.HitActor (Collision|BreakHitResult _outhit))))
    (if (not _success)
      (Class|BPITrolleyInterface|PossessTrolley(Message) (.HitActor (Collision|BreakHitResult _outhit)) self)
      (Rendering|SetVisibility (Variables|Character|GetMesh) false true)
      (Collision|SetCollisionEnabled (Variables|Collision|GetCapsuleComponent) "NoCollision"))))

(event Input|EnhancedActionEvents|EnhancedInputActionIA_Boost
  (params (ActionValue :type Boolean) (ElapsedSeconds :type Float%20%28double-precision%29) (TriggeredSeconds :type Float%20%28double-precision%29) (InputAction :type Input%20Action%20Object%20Reference :default "/Game/Blueprints/_Game/Input/Inputs/Abilities/IA_Boost.IA_Boost"))
  (bind _charactermovement (Variables|Character|GetCharacterMovement))
  (:Triggered
    (Variables|/Script/Engine.CharacterMovementComponent|SetMaxWalkSpeed _charactermovement (Variables|Default|GetSprintSpeed)))
  (:Completed
    (Variables|/Script/Engine.CharacterMovementComponent|SetMaxWalkSpeed _charactermovement (Variables|Default|GetWalkSpeed))))

(event EventReturntoPlayer
  (params (CurrentUser :type Pawn%20Object%20Reference))
  (Variables|Default|SetCurrent%20User CurrentUser)
  (Pawn|Possess (Game|GetPlayerController 0) self))

(event EventPossessed
  (params (NewController :type Controller%20Object%20Reference))
  (bind _current_user (Variables|Default|GetCurrent%20User)
    (:then
      (bind _trolleyhandlebar (Class|BPITrolleyInterface|GetTrolleyInfo(Message) _current_user))
      (Transformation|SetActorLocationAndRotation _trolleyhandlebar (Math|Rotator|MakeRotator 0.0 0.0 (.yaw (Transformation|GetActorRotation _current_user))) false true)
      (Rendering|SetVisibility (Variables|Character|GetMesh) true true)
      (Collision|SetCollisionEnabled (Variables|Collision|GetCapsuleComponent) "QueryAndProbe"))
    (:else)))

(fn ConstructionScript)