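; BP_Marker is a numbered car park marker that can randomly spawn a trolley bay.
; On BeginPlay, a random roll gives roughly a one in ten chance to spawn BP_TrolleyBay at the Arrow component's world location and rotation.
; The construction script writes Number to the TextRender, or hides the text when Number is zero.
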(event EventBeginPlay
  (bind _arrow (Variables|Default|GetArrow))
  (bind _returnvalue (Transformation|GetWorldRotation _arrow))
  (if (> (Math|Random|RandomFloatinRange 0.0 5e+01) 45.0)
    (Game|SpawnActorfromClass "/Game/Blueprints/TrolleyBay/BP_TrolleyBay.BP_TrolleyBay_C" (Math|Transform|MakeTransform (Transformation|GetWorldLocation _arrow) (Math|Rotator|MakeRotator (.roll _returnvalue) (.pitch _returnvalue) (.yaw _returnvalue)) "1.000000,1.000000,1.000000") "Undefined" "MultiplyWithRoot" 0 0)))

(fn ConstructionScript
  (bind _textrender (Variables|Default|GetTextRender))
  (bind _number (Variables|Default|GetNumber))
  (if (== _number 0)
    (Rendering|SetVisibility _textrender false false)
    (else
      (Rendering|Components|TextRender|SetText _textrender (Utilities|Text|ToText(Integer) _number)))))