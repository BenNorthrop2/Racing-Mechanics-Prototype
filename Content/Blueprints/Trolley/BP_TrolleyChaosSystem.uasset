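; BP_TrolleyChaosSystem is a player-drivable trolley pawn built on a vehicle movement component.
; Enhanced Input move actions feed steering and throttle, while look actions drive controller yaw and pitch.
; On possession, it shows the skeletal mesh and activates the camera for player control, and hides and deactivates them for any other controller.
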(event Input|EnhancedActionEvents|EnhancedInputActionIA_Look
  (params (ActionValue :type Vector%202D%20Structure) (ElapsedSeconds :type Float%20%28double-precision%29) (TriggeredSeconds :type Float%20%28double-precision%29) (InputAction :type Input%20Action%20Object%20Reference :default "/Game/Blueprints/Game/Input/Inputs/Movement/IA_Look.IA_Look"))
  (Pawn|Input|AddControllerYawInput (.x ActionValue))
  (Pawn|Input|AddControllerPitchInput (.y ActionValue)))

(event Input|EnhancedActionEvents|EnhancedInputActionIA_Move
  (params (ActionValue :type Vector%202D%20Structure) (ElapsedSeconds :type Float%20%28double-precision%29) (TriggeredSeconds :type Float%20%28double-precision%29) (InputAction :type Input%20Action%20Object%20Reference :default "/Game/Blueprints/Game/Input/Inputs/Movement/IA_Move.IA_Move"))
  (bind _vehiclemovementcomponent (Variables|Default|GetVehicleMovementComponent))
  (Class|ChaosVehicleMovementComponent|SetSteeringInput _vehiclemovementcomponent (.x ActionValue))
  (Class|ChaosVehicleMovementComponent|SetThrottleInput _vehiclemovementcomponent (.y ActionValue)))

(event EventPossessed
  (params (NewController :type Controller%20Object%20Reference))
  (if (Pawn|IsPlayerControlled)
    (Rendering|SetVisibility (Variables|Default|GetSkeletalMesh) true false)
    (Components|Activation|SetActive (Variables|Default|GetCamera) true false)
    (else
      (Rendering|SetVisibility (Variables|Default|GetSkeletalMesh) false false)
      (Components|Activation|SetActive (Variables|Default|GetCamera) false false))))

(fn ConstructionScript)