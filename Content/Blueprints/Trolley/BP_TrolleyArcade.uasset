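; Drivable arcade shopping trolley pawn that the player possesses, with boost, flip reset and exit back to the player pawn.
; While player-possessed, a looping timer drives physics: four wheel traces apply suspension and acceleration forces and update grounded state.
; Steering applies torque to the collision body.
; A debug key tows an overlapped trolley via physics constraint, passing it reduced steering; damped suspension and lateral friction functions are unused.
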(event OnComponentBeginOverlap(TrolleyDetectCol)
  (params (OverlappedComponent :type Primitive%20Component%20Object%20Reference) (OtherActor :type Actor%20Object%20Reference) (OtherComp :type Primitive%20Component%20Object%20Reference) (OtherBodyIndex :type Integer) (bFromSweep :type Boolean) (SweepResult :type Hit%20Result%20Structure%20%28by%20ref%29))
  ;[0.8281 0.6033 0 0.5] Trolley Connection (Improve Later)
  ;;[0.5729 0.2017 0 0.5] Get Overlapped Trolley Reference (Replace)
  (if (!= OtherActor self)
    (bind _asbp_trolley_arcade (Utilities|Casting|CastToBP_TrolleyArcade OtherActor))
    (Utilities|IsValid _asbp_trolley_arcade
      (:Is%20Valid
        (Variables|References|SetConnectedTrolley _asbp_trolley_arcade)
        (Variables|Checks|SetCanConnect true))
      (:Is%20Not%20Valid
        (Variables|Checks|SetCanConnect false)))))

(event OnComponentEndOverlap(TrolleyDetectCol)
  (params (OverlappedComponent :type Primitive%20Component%20Object%20Reference) (OtherActor :type Actor%20Object%20Reference) (OtherComp :type Primitive%20Component%20Object%20Reference) (OtherBodyIndex :type Integer))
  ;[0.8281 0.6033 0 0.5] Trolley Connection (Improve Later)
  (if (!= OtherActor self)
    (Variables|References|SetConnectedTrolley 0)))

(event Custom|HandlePhysics
  ;[0 0.15 0.004487 0.5] Handles Physics
  (if (Variables|Checks|GetShouldRunPhysics?)
    (Suspension|PhysicsUpdate)
    (bind _connectedtrolley (Variables|References|GetConnectedTrolley)
      (:then
        (Variables|BP_TrolleyArcade_C|SetShouldRunPhysics? _connectedtrolley true)
        (bind _output_get (Variables|BP_TrolleyArcade_C|SetSteerInput _connectedtrolley (/ (Variables|Inputs|GetSteerInput) 1e+01)))
        (Acceleration|HandleSteering _connectedtrolley _output_get))
      (:else))))

(event Input|EnhancedActionEvents|EnhancedInputActionIA_Look
  (params (ActionValue :type Vector%202D%20Structure) (ElapsedSeconds :type Float%20%28double-precision%29) (TriggeredSeconds :type Float%20%28double-precision%29) (InputAction :type Input%20Action%20Object%20Reference :default "/Game/Blueprints/_Game/Input/Inputs/Movement/IA_Look.IA_Look"))
  ;[1 0.06306 0.000236 0.5 24] Inputs And Controls
  ;;[1 0.000747 9e-06 0.5] Camera Controls
  (Pawn|Input|AddControllerYawInput (.x ActionValue))
  (Pawn|Input|AddControllerPitchInput (.y ActionValue)))

(event Input|EnhancedActionEvents|EnhancedInputActionIA_ResetTrolley
  (params (ActionValue :type Boolean) (ElapsedSeconds :type Float%20%28double-precision%29) (TriggeredSeconds :type Float%20%28double-precision%29) (InputAction :type Input%20Action%20Object%20Reference :default "/Game/Blueprints/_Game/Input/Inputs/Abilities/IA_ResetTrolley.IA_ResetTrolley"))
  (Utility|CheckFlipped))

(event Input|EnhancedActionEvents|EnhancedInputActionIA_Boost
  (params (ActionValue :type Boolean) (ElapsedSeconds :type Float%20%28double-precision%29) (TriggeredSeconds :type Float%20%28double-precision%29) (InputAction :type Input%20Action%20Object%20Reference :default "/Game/Blueprints/_Game/Input/Inputs/Abilities/IA_Boost.IA_Boost"))
  ;[1 0.06306 0.000236 0.5 24] Inputs And Controls
  ;;[1 0 0.4097 0.5] Boost Trolley For A Second
  (Variables|Acceleration|SetSpeedMultiplier 2.0)
  (Utilities|FlowControl|Delay 1.0)
  (Variables|Acceleration|SetSpeedMultiplier 1.0))

(event Input|EnhancedActionEvents|EnhancedInputActionIA_Interact
  (params (ActionValue :type Boolean) (ElapsedSeconds :type Float%20%28double-precision%29) (TriggeredSeconds :type Float%20%28double-precision%29) (InputAction :type Input%20Action%20Object%20Reference :default "/Game/Blueprints/_Game/Input/Inputs/Abilities/IA_Interact.IA_Interact"))
  ;[0.134 0.6667 0.1548 0.5] Return To Player Pawn
  (Pawn|Possess (Game|GetPlayerController 0) (Variables|References|GetPlayerRef)))

(event Input|EnhancedActionEvents|EnhancedInputActionIA_Steer
  (params (ActionValue :type Float%20%28double-precision%29) (ElapsedSeconds :type Float%20%28double-precision%29) (TriggeredSeconds :type Float%20%28double-precision%29) (InputAction :type Input%20Action%20Object%20Reference :default "/Game/Blueprints/_Game/Input/Inputs/Movement/IA_Steer.IA_Steer"))
  (Variables|Inputs|SetSteerInput ActionValue)
  (if (Variables|Checks|GetIsGrounded)
    (Acceleration|HandleSteering (Variables|Inputs|GetSteerInput))))

(event Input|EnhancedActionEvents|EnhancedInputActionIA_Accelerate
  (params (ActionValue :type Float%20%28double-precision%29) (ElapsedSeconds :type Float%20%28double-precision%29) (TriggeredSeconds :type Float%20%28double-precision%29) (InputAction :type Input%20Action%20Object%20Reference :default "/Game/Blueprints/_Game/Input/Inputs/Movement/IA_Accelerate.IA_Accelerate"))
  (Variables|Inputs|SetAccelInput (Math|Interpolation|FInterpTo (Variables|Inputs|GetAccelInput) (Math|Float|SelectFloat ActionValue 0.0 (Variables|Checks|GetIsGrounded)) (Utilities|Time|GetWorldDeltaSeconds) (Variables|Acceleration|GetAccelerationIncrease))))

(event Input|EnhancedActionEvents|EnhancedInputActionIA_Reverse
  (params (ActionValue :type Float%20%28double-precision%29) (ElapsedSeconds :type Float%20%28double-precision%29) (TriggeredSeconds :type Float%20%28double-precision%29) (InputAction :type Input%20Action%20Object%20Reference :default "/Game/Blueprints/_Game/Input/Inputs/Movement/IA_Reverse.IA_Reverse"))
  (Variables|Inputs|SetAccelInput (Math|Interpolation|FInterpTo (Variables|Inputs|GetAccelInput) (Math|Float|SelectFloat ActionValue 0.0 (Variables|Checks|GetIsGrounded)) (Utilities|Time|GetWorldDeltaSeconds) (Variables|Acceleration|GetAccelerationIncrease))))

(event EventPossessed
  (params (NewController :type Controller%20Object%20Reference))
  ;[0.15 0.15 0.15 0.5] Check If Is Controlled, Toggle Physics depending on result
  (if (Pawn|IsPlayerControlled)
    (Variables|Checks|SetShouldRunPhysics? true)
    (bind _returnvalue (Utilities|Time|SetTimerbyEvent (EventDispatchers|CreateEvent :!event Custom|HandlePhysics) 0.01 true))
    (Variables|Default|SetPhysicsTimer _returnvalue)
    (else
      (Variables|Checks|SetShouldRunPhysics? false))))

(event EventUnpossessed
  (params (OldController :type Controller%20Object%20Reference))
  ;[0.15 0.15 0.15 0.5] Once UnPossessed Disable Physics
  (Variables|Checks|SetShouldRunPhysics? false)
  (Utilities|Time|ClearandInvalidateTimerbyHandle (Variables|Default|GetPhysicsTimer)))

(event EventDestroyed
  ;[0.134 0.6667 0.1548 0.5] Return To Player Pawn
  (Pawn|Possess (Game|GetPlayerController 0) (Variables|References|GetPlayerRef)))

(event EventUnPossessTrolley
  ;[0.134 0.6667 0.1548 0.5] Return To Player Pawn
  (Pawn|Possess (Game|GetPlayerController 0) (Variables|References|GetPlayerRef)))

(event Input|KeyboardEvents|DebugKeyT
  (params (Key :type Key%20Structure :default "None") (ActionValue :type Input%20Action%20Value%20Structure))
  (bind _skeletalmesh (Variables|Default|GetSkeletalMesh))
  (bind _connectedtrolley (Variables|References|GetConnectedTrolley))
  (bind _connectedtrolley_2 (Variables|References|GetConnectedTrolley))
  (bind _returnvalue (Transformation|GetSocketTransform _skeletalmesh "TrolleyConnectionPos" "RTS_World"))
  (bind _trolleycollision (Variables|BP_TrolleyArcade_C|GetTrolleyCollision _connectedtrolley))
  ;[0.8281 0.6033 0 0.5] Trolley Connection (Improve Later)
  ;;[0.7917 0.348 0 0.5] Toggle Connection Between Trolleys
  (:Pressed
    (Utilities|IsValid (Variables|References|GetConnectedTrolley)
      (:Is%20Valid
        (if (Variables|Checks|GetCanConnect)
          (Variables|Checks|SetCanConnect false)
          (Transformation|SetRelativeLocationAndRotation _trolleycollision (.location _returnvalue) (.rotation _returnvalue) false false)
          (Class|PhysicsConstraintComponent|SetConstrainedComponents (Variables|Default|GetTrolleyTow) (Variables|Default|GetTrolleyCollision) "None" _trolleycollision "None")
          (Variables|BP_TrolleyArcade_C|SetDoorOpen? _connectedtrolley_2 true)
          (else
            (Variables|Checks|SetCanConnect true)
            (Class|PhysicsConstraintComponent|BreakConstraint (Variables|Default|GetTrolleyTow))
            (Transformation|SetRelativeLocationAndRotation _trolleycollision (.location _returnvalue) (.rotation _returnvalue) false false)
            (Variables|BP_TrolleyArcade_C|SetDoorOpen? _connectedtrolley_2 false)))))))

(fn ConstructionScript)

(fn HandleSuspension
  (params (CurrentWheel :type Scene%20Component%20Object%20Reference) (SuspensionDistance :type Float%20%28single-precision%29))
  (bind _returnvalue (Transformation|GetWorldLocation CurrentWheel))
  ;[1 0 0 0.5] Traces Down From Each Wheel
  (bind _outhit (Collision|LineTraceByChannel _returnvalue (+ _returnvalue (* (Math|Vector|GetUpVector CurrentWheel) SuspensionDistance)) "TraceTypeQuery1" false 0 "ForOneFrame"))
  (if (.bBlockingHit (Collision|BreakHitResult _outhit))
    ;[0.01744 0.3141 1 0.5] Checks The Rotation, Prevents Suspension on Side.
    (if (> (Math|Vector|DotProduct (Transformation|GetActorUpVector) "0.000000,0.000000,1.000000") 0.8)
      (LocalVariables|SetDistance (.Distance (Collision|BreakHitResult _outhit)))
      (Class|PrimitiveComponent|AddForceatLocation (Variables|Default|GetTrolleyCollision) (* (- 1.0 (Math|Float|NormalizetoRange (LocalVariables|GetDistance) 3e+01 35.0)) (Math|Vector|GetUnitDirection(Vector) (.TraceEnd (Collision|BreakHitResult _outhit)) (.TraceStart (Collision|BreakHitResult _outhit))) (Variables|Suspension|GetSuspensionForce) (Utilities|Time|GetWorldDeltaSeconds)) (Transformation|GetWorldLocation CurrentWheel) "None")
      (Acceleration|HandleAcceleration CurrentWheel)
      (return 1))
    (else
      ;[0.2166 0.3692 1 0.5] Check Acceleration In Air, Prevents Flying.
      (Acceleration|HandleAcceleration CurrentWheel)
      (return 0))))

(fn CalculateAcceleration
  (Variables|Inputs|SetAccelerationForce (* (Math|Float|Lerp 0.0 (Variables|VisualsRotation|GetWheelRotationSpeed) (Variables|Inputs|GetAccelInput)) (Variables|Inputs|GetAccelInput)))
  (Variables|Inputs|SetAccelInput (Math|Interpolation|FInterpTo (Variables|Inputs|GetAccelInput) 0.0 (Utilities|Time|GetWorldDeltaSeconds) (Variables|Acceleration|GetDeAcceleartionSpeed)))
  (Visuals|CalculateWheelRotation (Variables|Inputs|GetAccelerationForce) (Variables|VisualsRotation|GetWheelRotationSpeed)))

(fn HandleAcceleration
  (params (CurrentWheel :type Scene%20Component%20Object%20Reference))
  (bind _trolleycollision (Variables|Default|GetTrolleyCollision))
  (Class|PrimitiveComponent|AddForceatLocation (Variables|Default|GetTrolleyCollision) (* (Math|Vector|GetForwardVector _trolleycollision) (Variables|Acceleration|GetAccelerationSpeed) (Variables|Inputs|GetAccelInput) (Physics|GetMass _trolleycollision) (Variables|Acceleration|GetSpeedMultiplier)) (Transformation|GetWorldLocation CurrentWheel) "None"))

(fn CalculateWheelRotation
  (params (Force :type Float%20%28double-precision%29) (Wheel%20Rotation%20Speed :type Float%20%28double-precision%29))
  (Variables|VisualsRotation|SetWheelRotation Wheel%20Rotation%20Speed))

(fn CheckFlipped
  (if (and (< (Math|Vector|DotProduct (Transformation|GetActorUpVector) "0.000000,0.000000,1.000000") 0.8) (Variables|Checks|GetIsGrounded))
    (Variables|Checks|SetIsFlipped true)
    (Utilities|IsValid (Variables|References|GetPlayerRef)
      (:Is%20Valid
        (Pawn|Possess (Game|GetPlayerController 0) (Variables|References|GetPlayerRef))
        (Variables|References|SetPlayerRef 0))
      (:Is%20Not%20Valid
        _))
    (Utility|ResetPosition)
    (else
      (Variables|Checks|SetIsFlipped false))))

(fn ResetPosition
  (bind _trolleycollision (Variables|Default|GetTrolleyCollision))
  (Transformation|SetActorTransform (Math|Transform|MakeTransform (+ (Transformation|GetActorLocation) "0,0,50.000000") (Math|Rotator|MakeRotator 0.0 0.0 (.yaw (Transformation|GetActorRotation)))) false true)
  (Class|PrimitiveComponent|SetPhysicsAngularVelocityinDegrees _trolleycollision "0, 0, 0" false "None")
  (Physics|SetPhysicsLinearVelocity _trolleycollision "0, 0, 0" false "None"))

(fn CalculateRotatorDirection
  (Variables|VisualsRotation|SetRotatorRotation (Math|Interpolation|FInterpTo (.yaw (Variables|/Script/Engine.SceneComponent|GetRelativeRotation (Variables|Default|GetTrolleyCollision))) (Math|Float|Clamp(Float) (Class|KismetAnimationLibrary|CalculateDirection (Transformation|GetVelocity) (Math|Rotator|MakeRotator 0.0 0.0 (.yaw (Transformation|GetWorldRotation (Variables|Default|GetTrolleyCollision))))) -1.0) (Utilities|Time|GetWorldDeltaSeconds) 1.0)))

(fn HandleSuspensionWDamper
  (params (CurrentWheel :type Scene%20Component%20Object%20Reference) (SuspensionDistance :type Float%20%28single-precision%29))
  (bind _returnvalue (Transformation|GetWorldLocation CurrentWheel))
  (bind _returnvalue_2 (Math|Vector|GetUpVector CurrentWheel))
  (bind _returnvalue_3 (Transformation|GetWorldLocation CurrentWheel))
  (bind _outhit (Collision|LineTraceByChannel _returnvalue (+ _returnvalue (* (Math|Vector|GetUpVector CurrentWheel) SuspensionDistance)) "TraceTypeQuery1" false 0 "ForOneFrame"))
  (if (.bBlockingHit (Collision|BreakHitResult _outhit))
    (LocalVariables|SetDistance (.Distance (Collision|BreakHitResult _outhit)))
    (bind _returnvalue_4 (Class|PrimitiveComponent|GetPhysicsLinearVelocityatPoint (Variables|Default|GetTrolleyCollision) (Transformation|GetWorldLocation CurrentWheel) "None"))
    (Class|PrimitiveComponent|AddForceatLocation (Variables|Default|GetTrolleyCollision) (Math|Vector|SelectVector (+ (* (- 1.0 (Math|Float|NormalizetoRange (LocalVariables|GetDistance) 18.0 2e+01)) _returnvalue_2 (Variables|Suspension|GetSuspensionForce)) (* _returnvalue_2 (* (* (Math|Vector|DotProduct _returnvalue_4 (Math|Vector|GetUpVector CurrentWheel)) (Variables|Suspension|GetSuspensionDamp)) -1.0))) "0, 0, 0" (< (- (LocalVariables|GetDistance) SuspensionDistance) 0.5)) _returnvalue_3 "None")
    (Rendering|Debug|DrawDebugArrow _returnvalue_3 (+ _returnvalue_3 (* (+ (* (- 1.0 (Math|Float|NormalizetoRange (LocalVariables|GetDistance) 18.0 2e+01)) _returnvalue_2 (Variables|Suspension|GetSuspensionForce)) (* _returnvalue_2 (* (* (Math|Vector|DotProduct _returnvalue_4 (Math|Vector|GetUpVector CurrentWheel)) (Variables|Suspension|GetSuspensionDamp)) -1.0))) 0.001)) 0.0 "(R=0.024221,G=1.000000,B=0.244189,A=1.000000)" 0.0 0.0)
    (Acceleration|HandleAcceleration CurrentWheel)
    (return 1)
    (else
      (Acceleration|HandleAcceleration CurrentWheel)
      (return 0))))

(fn PhysicsUpdate
  (bind _outhit (Suspension|HandleSuspension (Variables|Default|GetFL_Wheel) (Variables|Suspension|GetFrontSuspensionDistance)))
  (bind _outhit_2 (Suspension|HandleSuspension (Variables|Default|GetFR_Wheel) (Variables|Suspension|GetFrontSuspensionDistance)))
  (bind _outhit_3 (Suspension|HandleSuspension (Variables|Default|GetBL_Wheel) (Variables|Suspension|GetRearSuspensionDistance)))
  (bind _outhit_4 (Suspension|HandleSuspension (Variables|Default|GetBR_Wheel) (Variables|Suspension|GetRearSuspensionDistance)))
  (Acceleration|CalculateAcceleration)
  (Visuals|CalculateRotatorDirection)
  (Variables|Checks|SetIsGrounded (>= (+ (+ _outhit_4 _outhit_3) (+ _outhit_2 _outhit)) 1)))

(fn AddSuspensionForce
  (params (CurrentWheel :type Scene%20Component%20Object%20Reference) (InputPin :type Float%20%28single-precision%29) (InputPin2 :type Vector) (InputPin1 :type Vector))
  (LocalVariables|SetDistance InputPin)
  (Class|PrimitiveComponent|AddForceatLocation (Variables|Default|GetTrolleyCollision) (* (- 1.0 (Math|Float|NormalizetoRange (LocalVariables|GetDistance) 3e+01 35.0)) (Math|Vector|GetUnitDirection(Vector) InputPin2 InputPin1) (Variables|Suspension|GetSuspensionForce)) (Transformation|GetWorldLocation CurrentWheel) "None")
  (Acceleration|HandleAcceleration CurrentWheel))

(fn HandleSteering
  (params (Steer%20Input :type Float%20%28double-precision%29))
  (Class|PrimitiveComponent|AddTorqueinRadians (Variables|Default|GetTrolleyCollision) (Math|Vector|MakeVector 0.0 0.0 (* Steer%20Input (Variables|Acceleration|GetTurnSpeed) (Physics|GetMass (Variables|Default|GetTrolleyCollision)) 1e+02)) "None" false))

(fn GetSlopeAngle
  (bind _trolleycollision (Variables|Default|GetTrolleyCollision))
  (bind _trolleycollision_2 (Variables|Default|GetTrolleyCollision))
  (bind _returnvalue (Transformation|GetWorldLocation _trolleycollision))
  (bind (_outhit _returnvalue_2) (Collision|LineTraceByChannel _returnvalue (+ _returnvalue (* (Math|Vector|GetUpVector _trolleycollision) -1e+02)) "TraceTypeQuery1" false 0 "ForOneFrame"))
  (if _returnvalue_2
    (return (.OutSlopeRollDegreeAngle (Class|KismetMathLibrary|GetSlopeDegreeAngles (Math|Vector|GetRightVector _trolleycollision_2) (.ImpactNormal (Collision|BreakHitResult _outhit)) (Math|Vector|GetUpVector _trolleycollision_2))))))

(fn CalculateLateralFriction
  (params (CurrentWheel :type Scene%20Component%20Object%20Reference))
  (bind _returnvalue (Transformation|GetWorldLocation CurrentWheel))
  (bind _returnvalue_2 (Class|PrimitiveComponent|GetPhysicsLinearVelocityatPoint (Variables|Default|GetTrolleyCollision) (Transformation|GetWorldLocation CurrentWheel) "None"))
  (Class|PrimitiveComponent|AddForceatLocation (Variables|Default|GetTrolleyCollision) (* (/ (* (Math|Vector|DotProduct _returnvalue_2 (Math|Vector|GetRightVector CurrentWheel)) -1.0 (Variables|Default|GetTireGrip)) (Utilities|Time|GetWorldDeltaSeconds)) 5.0 (Math|Vector|GetRightVector CurrentWheel)) _returnvalue "None")
  (Rendering|Debug|DrawDebugArrow _returnvalue (+ _returnvalue (* (* (/ (* (Math|Vector|DotProduct _returnvalue_2 (Math|Vector|GetRightVector CurrentWheel)) -1.0 (Variables|Default|GetTireGrip)) (Utilities|Time|GetWorldDeltaSeconds)) 5.0 (Math|Vector|GetRightVector CurrentWheel)) 0.1)) 25.0 "(R=0.000000,G=1.000000,B=0.082267,A=1.000000)" 0.0 1.0))

(fn GetTrolleyLinks
  (return 0 0))