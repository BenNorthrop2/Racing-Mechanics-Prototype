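; Trolley manager component that keeps an ordered chain of linked trolleys, starting with its owner.
; Attaching box-searches near a given trolley, snaps the nearest valid one to its connection socket, joins them with a physics constraint and appends the found trolley's chain.
; Detaching breaks the last link, teleports that trolley to its own socket and removes it.
; Scaled acceleration and steering input is relayed to following trolleys through interface messages.
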(event EventBeginPlay
  (Utilities|Array|AddUnique (Variables|Default|GetChainArray) (Components|GetOwner)))

(fn GetLastTrolley
  (bind _chainarray (Variables|Default|GetChainArray))
  (return (Utilities|Array|Get(acopy) _chainarray (Utilities|Array|LastIndex _chainarray))))

(fn AttemptConnect
  (params (LastTrolley :type Actor%20Object%20Reference))
  (bind (_success _foundtrolley) (CallFunction|FindConnectableTrolley LastTrolley))
  (if _success
    (LocalVariables|SetFoundTrolley _foundtrolley)
    (bind _canconnect_ (Class|BPITrolleyInterface|ValidateConection(Message) (LocalVariables|GetFoundTrolley)))
    (if _canconnect_
      (bind _collisioncomp (Class|BPITrolleyInterface|GetCollision(Message) (LocalVariables|GetFoundTrolley)))
      (bind (_trolleysearchlocation _trolleyhandlebar _trolleysearchrotation _constraint _trolleycollision _mesh) (Class|BPITrolleyInterface|GetTrolleyInfo(Message) LastTrolley))
      (Utilities|IsValid _collisioncomp
        (:Is%20Valid
          (Transformation|SetRelativeLocationAndRotation _collisioncomp (.location (Transformation|GetSocketTransform _mesh "TrolleyConnectionPos" "RTS_World")) (.rotation (Transformation|GetSocketTransform _mesh "TrolleyConnectionPos" "RTS_World")) false false)
          (Class|PhysicsConstraintComponent|SetConstrainedComponents _constraint _trolleycollision "None" _collisioncomp "None")
          (bind _chainarray (Class|BPITrolleyInterface|GetChainArray(Message) (LocalVariables|GetFoundTrolley)))
          (Utilities|Array|AppendArray (Variables|Default|GetChainArray) _chainarray)
          (Class|BPITrolleyInterface|OnConnected(Message) (LocalVariables|GetFoundTrolley) (Components|GetOwner)))))))

(fn DettachFrontTrolley
  (bind _chainarray (Variables|Default|GetChainArray))
  (bind _chainarray_2 (Variables|Default|GetChainArray))
  (bind _returnvalue (Utilities|Array|LastIndex _chainarray_2))
  (bind _output (Utilities|Array|Get(acopy) _chainarray_2 _returnvalue))
  (if (> (Utilities|Array|Length (Variables|Default|GetChainArray)) 1)
    (bind _constraint (Class|BPITrolleyInterface|GetTrolleyInfo(Message) (Utilities|Array|Get(acopy) _chainarray (- (Utilities|Array|LastIndex _chainarray) 1))))
    (Utilities|IsValid _constraint
      (:Is%20Valid
        (Class|PhysicsConstraintComponent|BreakConstraint _constraint)
        (CallFunction|SetTrolleyLocationAfter _output)
        (Class|BPITrolleyInterface|OnDisconnected(Message) _output)
        (Utilities|Array|RemoveItem (Variables|Default|GetChainArray) _output)))))

(fn FindConnectableTrolley
  (params (Trolley :type Object%20Object%20Reference))
  (bind (_trolleysearchlocation _trolleyhandlebar _trolleysearchrotation) (Class|BPITrolleyInterface|GetTrolleyInfo(Message) Trolley))
  (bind (_outactors _returnvalue) (Collision|BoxOverlapActorsWithOrientation _trolleysearchlocation "32.000000,32.000000,32.000000" _trolleysearchrotation (Utilities|Array|MakeArray "ObjectTypeQuery7") 0))
  (if _returnvalue
    (if (Utilities|DoesObjectImplementInterface (.ReturnValue (Actor|FindNearestActor _trolleysearchlocation _outactors)) "/Game/Blueprints/Interfaces/BPI_TrolleyInterface.BPI_TrolleyInterface_C")
      (return true (.ReturnValue (Actor|FindNearestActor _trolleysearchlocation _outactors)))
      (else
        (return false 0)))
    (else
      (return false 0))))

(fn GetTrolleyNames
  (for _array_element (Variables|Default|GetChainArray)
    (Utilities|IsValid _array_element
      (:Is%20Valid
        (Development|PrintString (Utilities|GetDisplayName _array_element))))))

(fn SetTrolleyLocationAfter
  (params (Target :type Object%20Object%20Reference))
  (bind (_trolleysearchlocation _trolleyhandlebar _trolleysearchrotation _constraint _trolleycollision _mesh) (Class|BPITrolleyInterface|GetTrolleyInfo(Message) Target))
  (Transformation|SetRelativeLocationAndRotation _trolleycollision (Math|Vector|MakeVector (.X (Math|Vector|BreakVector (.location (Transformation|GetSocketTransform _mesh "TrolleyConnectionPos" "RTS_World")))) (.Y (Math|Vector|BreakVector (.location (Transformation|GetSocketTransform _mesh "TrolleyConnectionPos" "RTS_World")))) (.Z (Math|Vector|BreakVector (.location (Transformation|GetSocketTransform _mesh "TrolleyConnectionPos" "RTS_World"))))) (.rotation (Transformation|GetSocketTransform _mesh "TrolleyConnectionPos" "RTS_World")) false true))

(fn UpdateTrolleyMovements
  (params (AccelInput :type Float%20%28double-precision%29) (SteeringInput :type Float%20%28double-precision%29))
  (for (_array_element _array_index) (Variables|Default|GetChainArray)
    (if (> _array_index 0)
      (Class|BPITrolleyInterface|RecievePassiveInputs(Message) _array_element (* AccelInput 5e+02) SteeringInput))))