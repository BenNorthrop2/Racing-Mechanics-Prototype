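; BP_CollectionBay is a trolley collection bay that counts trolleys delivered into its trigger box.
; On BeginPlay it casts and stores the BP_GM_Timer game mode.
; When an overlapping actor implements BPI_TrolleyInterface, it tells the game mode to increment the trolley count, sends the trolley an unpossess message, then destroys it.
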(event OnComponentBeginOverlap(Box)
  (params (OverlappedComponent :type Primitive%20Component%20Object%20Reference) (OtherActor :type Actor%20Object%20Reference) (OtherComp :type Primitive%20Component%20Object%20Reference) (OtherBodyIndex :type Integer) (bFromSweep :type Boolean) (SweepResult :type Hit%20Result%20Structure%20%28by%20ref%29))
  (if (Utilities|DoesObjectImplementInterface OtherActor "/Game/Blueprints/Interfaces/BPI_TrolleyInterface.BPI_TrolleyInterface_C")
    (Utilities|IsValid OtherActor
      (:Is%20Valid
        (Default|CallHandleIncrementTrolley (Variables|Default|GetGameModeRef))
        (Class|BPITrolleyInterface|UnPossessTrolley(Message) OtherActor)
        (Actor|DestroyActor OtherActor)))))

(event EventBeginPlay
  (bind _asbp_gm_timer (Utilities|Casting|CastToBP_GM_Timer (Game|GetGameMode)))
  (Variables|Default|SetGameModeRef _asbp_gm_timer))

(fn ConstructionScript)