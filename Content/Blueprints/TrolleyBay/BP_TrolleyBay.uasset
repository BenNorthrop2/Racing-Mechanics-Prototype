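; Trolley bay actor that acts as a spawn point for trolleys.
; After a short delay on BeginPlay, it registers itself with the game mode through an interface and binds an event to the trolley-spawning handler.
; SpawnTrolley loops over a requested count, spawning BP_Trolley actors at random navigable points near the bay with random yaw and a debug print.
; The separate SpawnTrolleys and GetGameModeRef functions are empty stubs.
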(event EventSpawnTrolley
  (params (TrolleyCount :type Integer))
  (for _index (range 0 TrolleyCount)
    (bind _randomlocation (Class|NavigationSystemV1|GetRandomLocationinNavigableRadius (Transformation|GetActorLocation) 1e+02 0 0))
    (bind _returnvalue (Game|SpawnActorfromClass "/Game/Blueprints/Trolley/BP_Trolley.BP_Trolley_C" (Math|Transform|MakeTransform (Math|Vector|MakeVector (.x _randomlocation) (.y _randomlocation) (+ (.z _randomlocation) 1e+01)) (Math|Rotator|MakeRotator 0.0 0.0 (.yaw (Math|Random|RandomRotator false))) "1.000000,1.000000,1.000000") "AdjustIfPossibleButAlwaysSpawn" "MultiplyWithRoot" 0 0))
    (Utilities|IsValid _returnvalue
      (:Is%20Valid
        (Development|PrintString "Hello")))))

(event EventBeginPlay
  (bind _gamemode (Class|BPITrolleyBay|GetGameModeRef(Message) (Game|GetGameMode)))
  (Utilities|FlowControl|Delay 0.5)
  (Default|CallHandleGetTrolleyBays _gamemode self)
  (EventDispatchers|BindEventtoHandleSpawnTrolleys _gamemode (EventDispatchers|CreateEvent :!event SpawnTrolleys)))

(fn ConstructionScript)

(fn SpawnTrolleys
  (params (TrolleyCount :type Integer)))

(fn GetGameModeRef
  (return 0))